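; BP_Enemy_Custom is an enemy Blueprint that drops BP_Collectable pickups when it is destroyed.
; The Destroyed event runs a loop bounded by DropCollectable, spawning one pickup per iteration around the CollectableSpawnLocation component.
; Each pickup gets a random horizontal offset, made by flattening a random unit vector, and a random yaw.
; BeginPlay, overlap and Tick are disabled stubs, and the construction script only calls its parent.
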(event `self.ReceiveDestroyed`
  (for _ (range (+ (`self.DropCollectable`) 1))
    (`|SpawnActorFromClass` "/Game/BP_Collectable.BP_Collectable_C" (`KismetMathLibrary.MakeTransform` (+ (`SceneComponent.K2_GetComponentLocation` (`self.CollectableSpawnLocation`)) (* (`KismetMathLibrary.RandomUnitVector`) (100.0 100.0 0.0))) (`KismetMathLibrary.MakeRotator` 0.0 0.0 (`KismetMathLibrary.RandomFloatInRange` 0.0 999.0))) "Undefined" "OverrideRootScale" null null)))

(fn `UserConstructionScript`
  (`parent.UserConstructionScript`))